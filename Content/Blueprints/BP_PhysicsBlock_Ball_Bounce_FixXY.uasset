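; A physics ball block, named as a bouncing variant, whose mesh is locked to its starting X and Y so it moves only along the vertical axis.
; It records the static mesh's world location on BeginPlay, then every Tick resets X and Y to those values while keeping the current Z.
; The lock works by repositioning the mesh each frame, and any bounce behavior comes from outside these graphs.
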(event EventBeginPlay
  (|CallParentFunction)
  (Variables|Default|SetOriginalLocation (Transformation|GetWorldLocation (Variables|Default|GetStaticMesh))))

(event Collision|EventActorBeginOverlap
  (params (OtherActor :type Actor%20Object%20Reference))
  (|CallParentFunction OtherActor) ; This node is disabled and will not be called.\nDrag off pins to build functionality.
)

(event EventTick
  (params (DeltaSeconds :type Float%20%28single-precision%29))
  (bind _originallocation (Variables|Default|GetOriginalLocation))
  (bind (_x _y) (Math|Vector|BreakVector _originallocation))
  (|CallParentFunction DeltaSeconds)
  (Transformation|SetWorldLocation (Variables|Default|GetStaticMesh) (Math|Vector|MakeVector _x _y (.Z (Math|Vector|BreakVector (Transformation|GetWorldLocation (Variables|Default|GetStaticMesh))))) false false))

(fn ConstructionScript
  (|CallParentFunction))