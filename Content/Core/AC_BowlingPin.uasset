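; Bowling pin actor component that destroys its owner when the pin is knocked over or falls fast.
; It attaches a spawned BP_UpChecker and reads its up vector with owner speed to detect a toppled, slow-moving pin.
; Each state starts a retriggerable delay before destroying both actors; righting cancels the topple.
; The falling recovery branch clears IsFallDown rather than IsFalling, so that destruction still happens.
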(event EventTick
  (params (DeltaSeconds :type Float%20%28single-precision%29))
  (bind _returnvalue (Components|GetOwner))
  (bind _returnvalue_2 (Transformation|GetVelocity _returnvalue))
  (bind _returnvalue_3 (Math|Vector|VectorLength _returnvalue_2))
  (bind _returnvalue_4 (Utilities|String|ToString(Float) _returnvalue_3))
  (Utilities|FlowControl|Sequence
    (:then_0
      (if (and (< (Math|Vector|DotProduct (Transformation|GetActorUpVector (Variables|Default|GetUpChecker)) "0.000000,0.000000,1.000000") 0.4) (< _returnvalue_3 5e+01))
        (if (not (Variables|Default|GetIsFallDown))
          (Development|PrintString _returnvalue_4)
          (Development|PrintString "trigger")
          (Variables|Default|SetIsFallDown true)
          (Variables|Default|SetDuration 2.0)
          (Utilities|FlowControl|RetriggerableDelay (Variables|Default|GetDuration) :!label _label)
          (if (Variables|Default|GetIsFallDown)
            (Actor|DestroyActor (Components|GetOwner))
            (Actor|DestroyActor (Variables|Default|GetUpChecker))))
        (elif (Variables|Default|GetIsFallDown)
          (Development|PrintString _returnvalue_4)
          (Development|PrintString "recover")
          (Variables|Default|SetIsFallDown false)
          (Variables|Default|SetDuration 0.0)
          (goto _label))))
    (:then_1
      (if (< (.z (Transformation|GetVelocity (Components|GetOwner))) -1e+03)
        (if (not (Variables|Default|GetIsFalling))
          (Development|PrintString "trigger")
          (Variables|Default|SetIsFalling true)
          (Variables|Default|SetDuration 2.0)
          (Utilities|FlowControl|RetriggerableDelay (Variables|Default|GetDuration) :!label _label_2)
          (if (Variables|Default|GetIsFalling)
            (Actor|DestroyActor (Components|GetOwner))
            (Actor|DestroyActor (Variables|Default|GetUpChecker))))
        (elif (Variables|Default|GetIsFalling)
          (Development|PrintString "recover")
          (Variables|Default|SetIsFallDown false)
          (Variables|Default|SetDuration 0.0)
          (goto _label_2))))))

(event EventBeginPlay
  (bind _returnvalue (Game|SpawnActorfromClass "/Game/Core/BP_UpChecker.BP_UpChecker_C" (Math|Transform|MakeTransform (Math|Vector|MakeVector 0.0 0.0 5e+01) "0, 0, 0" "1.000000,1.000000,1.000000") "Undefined" "MultiplyWithRoot" 0 0))
  (bind _output_get (Variables|Default|SetUpChecker _returnvalue))
  (Transformation|AttachActorToActor _output_get (Components|GetOwner) "None" "KeepRelative" "KeepRelative" "KeepRelative" true))