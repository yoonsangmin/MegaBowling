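; First-person player pawn for a bowling game that moves, looks around with the mouse and launches balls.
; WASD builds an input vector that Tick rotates to the camera's yaw while pinning the pawn's height.
; Left-click press spawns a physics-disabled ball attached to the camera manager; release detaches and impulses it along the view, destroying it after a delay.
; The IA_PositiveMove Enhanced Input event only prints its value.
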(event Input|EnhancedActionEvents|EnhancedInputActionIA_PositiveMove
  (params (ActionValue :type Vector%202D%20Structure) (ElapsedSeconds :type Float%20%28double-precision%29) (TriggeredSeconds :type Float%20%28double-precision%29) (InputAction :type Input%20Action%20Object%20Reference :default "/Game/IA_PositiveMove.IA_PositiveMove"))
  (Development|PrintString (Utilities|String|ToString(Vector2d) ActionValue)))

(event EventTick
  (params (DeltaSeconds :type Float%20%28single-precision%29))
  (bind _returnvalue (Game|GetPlayerCameraManager 0))
  (bind _returnvalue_2 (Transformation|GetActorLocation))
  (bind _returnvalue_3 (Camera|GetCameraRotation _returnvalue))
  (bind _returnvalue_4 (Math|Vector|GetForwardVector _returnvalue_3))
  (if (< 0.0 (Math|Vector|DotProduct (Math|Vector|GetForwardVector _returnvalue_3) "0.000000,1.000000,0.000000"))
    (Variables|Default|SetIsFacingRight 1.0)
    (else
      (Variables|Default|SetIsFacingRight -1.0)))
  (Pawn|Input|AddMovementInput (Math|Vector|RotateVectorAroundAxis (Math|Vector|Normalize (Variables|Default|GetMoveKeyInput)) (* (Class|KismetMathLibrary|DegAcos (Math|Vector|DotProduct "1.000000,0.000000,0.000000" (Math|Vector|Normalize (Math|Vector|MakeVector (.x _returnvalue_4) (.y _returnvalue_4) 0.0)))) (Variables|Default|GetIsFacingRight)) "0.000000,0.000000,1.000000") (* DeltaSeconds (Variables|Default|GetMoveSpeed)) false)
  (Transformation|SetActorLocation (Math|Vector|MakeVector (.x _returnvalue_2) (.y _returnvalue_2) 125.0) false false))

(event Input|KeyboardEvents|W
  (params (Key :type Key%20Structure :default "None"))
  (:Pressed
    (Variables|Default|SetMoveKeyInput (+ (Variables|Default|GetMoveKeyInput) "1.000000,0.000000,0.000000")))
  (:Released
    (Variables|Default|SetMoveKeyInput (+ (Variables|Default|GetMoveKeyInput) "-1.000000,0.000000,0.000000"))))

(event Input|MouseEvents|LeftMouseButton
  (params (Key :type Key%20Structure :default "None"))
  (bind _returnvalue (Game|GetPlayerCameraManager 0))
  (bind _returnvalue_2 (Camera|GetCameraRotation _returnvalue))
  (bind _returnvalue_3 (Math|Vector|GetForwardVector _returnvalue_2))
  (:Pressed
    (bind _lastshotball (Variables|Default|GetLastShotBall)
      (:then)
      (:else
        (Variables|Default|SetIsReadyToShoot true)
        (Game|SpawnActorfromClass (Variables|Default|GetClass) (Math|Transform|MakeTransform (+ (Camera|GetCameraLocation _returnvalue) (* _returnvalue_3 1e+02)) "0, 0, 0" "1.000000,1.000000,1.000000") "Undefined" "MultiplyWithRoot" 0 0)
        (bind _output_get (Variables|Default|SetLastShotBall 0))
        (Physics|SetSimulatePhysics (Variables|/Script/Engine.StaticMeshActor|GetStaticMeshComponent _output_get) false)
        (Transformation|AttachActorToActor (Variables|Default|GetLastShotBall) (Game|GetPlayerCameraManager 0) "None" "KeepWorld" "KeepRelative" "KeepRelative" true))))
  (:Released
    (if (Variables|Default|GetIsReadyToShoot)
      (Variables|Default|SetIsReadyToShoot false)
      (Transformation|DetachFromActor (Variables|Default|GetLastShotBall) "KeepRelative" "KeepRelative" "KeepRelative")
      (Physics|SetSimulatePhysics (Variables|/Script/Engine.StaticMeshActor|GetStaticMeshComponent (Variables|Default|GetLastShotBall)) true)
      (Physics|AddImpulse (Variables|/Script/Engine.StaticMeshActor|GetStaticMeshComponent (Variables|Default|GetLastShotBall)) (* _returnvalue_3 (Variables|Default|GetPower)) "None" true)
      (Utilities|FlowControl|Delay 3.0)
      (Actor|DestroyActor (Variables|Default|GetLastShotBall)))))

(event Input|KeyboardEvents|S
  (params (Key :type Key%20Structure :default "None"))
  (:Pressed
    (Variables|Default|SetMoveKeyInput (+ (Variables|Default|GetMoveKeyInput) "-1.000000,0.000000,0.000000")))
  (:Released
    (Variables|Default|SetMoveKeyInput (+ (Variables|Default|GetMoveKeyInput) "1.000000,0.000000,0.000000"))))

(event Input|KeyboardEvents|A
  (params (Key :type Key%20Structure :default "None"))
  (:Pressed
    (Variables|Default|SetMoveKeyInput (+ (Variables|Default|GetMoveKeyInput) "0.000000,-1.000000,0.000000")))
  (:Released
    (Variables|Default|SetMoveKeyInput (+ (Variables|Default|GetMoveKeyInput) "0.000000,1.000000,0.000000"))))

(event Input|KeyboardEvents|D
  (params (Key :type Key%20Structure :default "None"))
  (:Pressed
    (Variables|Default|SetMoveKeyInput (+ (Variables|Default|GetMoveKeyInput) "0.000000,1.000000,0.000000")))
  (:Released
    (Variables|Default|SetMoveKeyInput (+ (Variables|Default|GetMoveKeyInput) "0.000000,-1.000000,0.000000"))))

(event Input|MouseEvents|Mouse2D
  (params (AxisValue :type Vector :default "0, 0, 0"))
  (bind _output_get (Variables|Default|SetRotation (Math|Rotator|MakeRotator 0.0 (Math|Float|Clamp(Float) (+ (* (Variables|Default|GetMouseScale) (.y AxisValue)) (.pitch (Variables|Default|GetRotation))) -89.99999 89.99999) (+ (* (Variables|Default|GetMouseScale) (.x AxisValue)) (.yaw (Variables|Default|GetRotation))))))
  (Pawn|SetControlRotation (Pawn|GetController) _output_get))

(fn ConstructionScript)