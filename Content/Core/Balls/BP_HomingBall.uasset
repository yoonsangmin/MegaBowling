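; BP_HomingBall is a bowling ball that makes a single homing turn toward a nearby pin after it is shot.
; OnShoot starts a looping timer that runs LockOn, which sphere-overlaps for actors with a BowlingPinComponent and keeps the nearest one in clear line of sight.
; Once a target exists, the timer stops and, after FollowDelay, a velocity-change impulse redirects the ball at the pin while preserving its speed.
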(event Custom|LockOn
  (bind _returnvalue (Transformation|GetVelocity))
  (bind _outactors (Collision|SphereOverlapActors (Transformation|GetActorLocation) (Variables|Default|GetLockOnRadius) (Utilities|Array|MakeArray "ObjectTypeQuery2" "ObjectTypeQuery4") "/Script/Engine.Actor"))
  (for _array_element _outactors
    (Utilities|IsValid (Actor|GetComponentbyClass _array_element "/Script/MegaBowling.BowlingPinComponent")
      (:Is%20Valid
        (bind (_outhit _returnvalue_2) (Collision|LineTraceForObjects (Transformation|GetActorLocation) (Transformation|GetActorLocation _array_element) (Utilities|Array|MakeArray "ObjectTypeQuery2" "ObjectTypeQuery4" "ObjectTypeQuery1") false 0 "None"))
        (if _returnvalue_2
          (if (== (.HitActor (Collision|BreakHitResult _outhit)) _array_element)
            (Utilities|IsValid (Variables|Default|GetTargetActor)
              (:Is%20Valid
                (if (< (Math|Vector|Distance(Vector) (Transformation|GetActorLocation (.HitActor (Collision|BreakHitResult _outhit))) (Transformation|GetActorLocation)) (Variables|Default|GetDistance))
                  (Variables|Default|SetTargetActor (.HitActor (Collision|BreakHitResult _outhit)))
                  (Variables|Default|SetDistance (Math|Vector|Distance(Vector) (Transformation|GetActorLocation (.HitActor (Collision|BreakHitResult _outhit))) (Transformation|GetActorLocation)))))
              (:Is%20Not%20Valid
                (bind _output_get (Variables|Default|SetTargetActor (.HitActor (Collision|BreakHitResult _outhit))))
                (Variables|Default|SetDistance (Math|Vector|Distance(Vector) (Transformation|GetActorLocation _output_get) (Transformation|GetActorLocation))))))))))
  (Utilities|IsValid (Variables|Default|GetTargetActor)
    (:Is%20Valid
      (Utilities|FlowControl|Sequence
        (:then_0
          (Utilities|Time|ClearandInvalidateTimerbyHandle (Variables|Default|GetLockOnHandle)))
        (:then_1
          (Utilities|FlowControl|Delay (Variables|Default|GetFollowDelay))
          (Physics|AddImpulse (Variables|Default|GetStaticMeshComponent) (- (* (Math|Vector|GetUnitDirection(Vector) (Transformation|GetActorLocation) (Transformation|GetActorLocation (Variables|Default|GetTargetActor))) (Math|Vector|VectorLength _returnvalue)) _returnvalue) "None" true))))))

(event EventOnShoot
  (bind _returnvalue (Utilities|Time|SetTimerbyEvent (delegate Custom|LockOn) (Variables|Default|GetLoopTime) true true))
  (Variables|Default|SetLockOnHandle _returnvalue))

(fn ConstructionScript)