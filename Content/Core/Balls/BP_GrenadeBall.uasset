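; Grenade ball that, once shot, waits for a fuse delay and then bursts into physical fragments.
; DestroyBall runs once, hiding the mesh and disabling its physics and collision, then spawns tagged fragments around the ball and impulses each along a random direction.
; After a further delay it destroys the spawned fragments and calls the parent DestroyBall to finish.
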(event EventDestroyBall
  (bind _staticmeshcomponent (Variables|Default|GetStaticMeshComponent))
  (Utilities|FlowControl|DoOnce false
    (:Completed
      (Utilities|FlowControl|Sequence
        (:then_0
          (Physics|SetSimulatePhysics _staticmeshcomponent false)
          (Collision|SetCollisionEnabled _staticmeshcomponent "NoCollision")
          (Rendering|SetVisibility _staticmeshcomponent false false))
        (:then_1
          (for _index (range 1 (Variables|Default|GetFragmentCount))
            (Variables|Default|SetRandomVector (Math|Random|RandomUnitVector))
            (bind _returnvalue (Game|SpawnActorfromClass (Variables|Default|GetFragmentClass) (Math|Transform|MakeTransform (+ (Transformation|GetActorLocation) (* (Variables|Default|GetRandomVector) 5.0)) "0, 0, 0" "1.000000,1.000000,1.000000") "Undefined" "MultiplyWithRoot" 0 0))
            (Utilities|Array|Add (Variables|/Script/Engine.Actor|GetTags _returnvalue) "Spawned")
            (Utilities|Array|Add (Variables|Default|GetSpawnedFragments) _returnvalue)
            (Physics|AddImpulse (Actor|GetComponentbyClass _returnvalue "/Script/Engine.StaticMeshComponent") (* (Variables|Default|GetRandomVector) (Variables|Default|GetImpulse)) "None" false)))
        (:then_2
          (Utilities|FlowControl|Delay (Variables|Default|GetExplosionAfterDelay))
          (Utilities|FlowControl|Sequence
            (:then_0
              (for _array_element (Variables|Default|GetSpawnedFragments)
                (Actor|DestroyActor _array_element)))
            (:then_1
              (|CallParentFunction))))))))

(event EventOnShoot
  (Utilities|FlowControl|Delay (Variables|Default|GetStartExplosionDelay))
  (Class|BowlingBall|DestroyBall))

(fn ConstructionScript)