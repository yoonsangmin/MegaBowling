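; BP_InvisibleWall is a wall that stays transparent until the player gets close, then fades into view.
; Each tick, a multi-sphere object trace at the player pawn's location uses OpacityThreshold as its radius.
; A hit on this wall sets the mesh material's Opacity parameter from the impact point's distance to the player, more opaque when nearer.
; Opacity resets to zero only when the trace hits nothing at all.
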(event EventBeginPlay)

(event Collision|EventActorBeginOverlap
  (params (OtherActor :type Actor%20Object%20Reference)))

(event EventTick
  (params (DeltaSeconds :type Float%20%28single-precision%29))
  (bind _returnvalue (Game|Player|GetPlayerPawn 0))
  (bind _returnvalue_2 (Transformation|GetActorLocation _returnvalue))
  (bind (_outhits _returnvalue_3) (Collision|MultiSphereTraceForObjects _returnvalue_2 _returnvalue_2 (Variables|Default|GetOpacityThreshold) (Utilities|Array|MakeArray "ObjectTypeQuery7") false 0 "None" false))
  (if _returnvalue_3
    (for _array_element _outhits
      (if (== (.HitActor (Collision|BreakHitResult _array_element)) self)
        (Rendering|Material|SetScalarParameterValueonMaterials (Variables|Debug|GetStaticMeshComponent) "Opacity" (- 1.0 (/ (Math|Vector|Distance(Vector) (.ImpactPoint (Collision|BreakHitResult _array_element)) (Transformation|GetActorLocation (Game|Player|GetPlayerPawn 0))) (Variables|Default|GetOpacityThreshold))))))
    (else
      (Rendering|Material|SetScalarParameterValueonMaterials (Variables|Debug|GetStaticMeshComponent) "Opacity" 0.0))))

(fn ConstructionScript)